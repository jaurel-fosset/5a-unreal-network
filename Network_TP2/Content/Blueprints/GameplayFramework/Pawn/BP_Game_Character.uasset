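; Player character Blueprint that fires through Shoot on the IA_Shoot input and visualizes client-predicted versus server-confirmed death.
; BeginPlay creates a dynamic Quinn material so death events can tint the mesh.
; Predicted death tints it blue and sets a flag, reverting after a brief delay if still unconfirmed.
; Confirmed death clears the flag, tints it red, then restores the color and moves the character to world origin, with debug prints throughout.
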(event `self.ReceiveBeginPlay`
  (bind _returnvalue (`KismetMaterialLibrary.CreateDynamicMaterialInstance` "/Game/Characters/Mannequins/Materials/Quinn/MI_Quinn_01.MI_Quinn_01" "DMI_Quinn_01"))
  (bind _output_get (set `self.MannequinColor` _returnvalue))
  (`PrimitiveComponent.SetMaterial` (`self.Mesh`) 0 _output_get))

(event `self.OnDeathBlueprintEvent`
  (if (`self.DeathPrediction`)
    (`KismetSystemLibrary.PrintString` "Client prediction confirmed")
    (set `self.DeathPrediction` false))
  (`MaterialInstanceDynamic.SetVectorParameterValue` (`self.MannequinColor`) "Paint Tint" (struct :`R` 1.0 :`G` 0.029369 :`B` 0.009235 :`A` 1.0))
  (`KismetSystemLibrary.PrintString` "Player death comfirmed by server")
  (`KismetSystemLibrary.Delay` 0.2)
  (`MaterialInstanceDynamic.SetVectorParameterValue` (`self.MannequinColor`) "Paint Tint" (struct :`R` 0.985971 :`G` 1.0 :`B` 0.950756 :`A` 1.0))
  (`self.K2_SetActorLocation` (0.0 0.0 0.0)))

(event `self.OnDeathPredictionBlueprintEvent`
  (`MaterialInstanceDynamic.SetVectorParameterValue` (`self.MannequinColor`) "Paint Tint" (struct :`G` 0.116311 :`B` 1.0 :`A` 1.0))
  (`KismetSystemLibrary.PrintString` "Player death predicted on client")
  (set `self.DeathPrediction` true)
  (`KismetSystemLibrary.Delay` 0.02)
  (if (`self.DeathPrediction`)
    (`MaterialInstanceDynamic.SetVectorParameterValue` (`self.MannequinColor`) "Paint Tint" (struct :`R` 0.985971 :`G` 1.0 :`B` 0.950756 :`A` 1.0))
    (set `self.DeathPrediction` false)
    (`KismetSystemLibrary.PrintString` "Player death not confirmed by server")))

(event `EnhancedInput|/Game/Input/Actions/IA_Shoot`
  (params (ActionValue :type Boolean) (ElapsedSeconds :type "Float (double-precision)") (TriggeredSeconds :type "Float (double-precision)") (InputAction :type "InputAction Object Reference" :default "/Game/Input/Actions/IA_Shoot.IA_Shoot"))
  (:`Triggered`
    (`self.Shoot`)))

(fn `UserConstructionScript`)